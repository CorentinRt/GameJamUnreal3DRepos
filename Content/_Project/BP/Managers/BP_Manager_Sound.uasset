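; Sound manager Blueprint that sets the base sound mix on BeginPlay and holds logic for fading background music.
; BeginPlay applies SCM_AudioMix and calls a play-music event, which is currently empty.
; Fade-in and fade-out events run three-second fades on valid audio components.
; A disconnected branch would spawn and fade in menu or game music by checking for the main menu level name, but never runs.
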(event `self.ReceiveBeginPlay`
  ;[0.4342 1 0.305] Begin Play
  (`GameplayStatics.SetBaseSoundMix` "/Game/_Project/Audio/SCM_AudioMix.SCM_AudioMix")
  (`self.CE_PlayMusic`))

(event `CE_PlayMusic`
  ;[0.9915 0.3387 1] Play Music
)

(event `CE_FadeInMusic`
  (params (Audio :type "AudioComponent Object Reference"))
  ;[1 0.527 0.9184] Fade In Out Music
  (`/Engine/EditorBlueprintResources/StandardMacros.IsValid` Audio
    (:`Is Valid`
      (`AudioComponent.FadeIn` Audio 3.0 1.0 0.0 "Linear"))))

(event `CE_FadeOutMusic`
  (params (Audio :type "AudioComponent Object Reference"))
  ;[1 0.527 0.9184] Fade In Out Music
  (`/Engine/EditorBlueprintResources/StandardMacros.IsValid` Audio
    (:`Is Valid`
      (`AudioComponent.FadeOut` Audio 3.0 0.0 "Linear"))))

(fn `UserConstructionScript`)