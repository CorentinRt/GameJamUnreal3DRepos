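; Manager for slow-motion quick-time events, auto-started three seconds after BeginPlay, broadcasting start, stop, win and lose events.
; Starting dilates global time and plays a timeline whose rate compensates for the slowdown; its end means a loss.
; After a dilation-compensated grace period, any player key except left mouse loses, while a separate success event wins.
; Either outcome unbinds the player controller's key event and restores normal time.
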(event `self.ReceiveBeginPlay`
  ;[0.397 1 0.4545] Begin Play
  (`|ExecutionSequence`
    (:`then_0`
      (bind _asbp_pc_player (cast `/Game/_Project/BP/Core/BP_PC_Player` (`GameplayStatics.GetPlayerController` 0)))
      (set `self.As BP PC Player` _asbp_pc_player))
    (:`then_1`
      (`KismetSystemLibrary.Delay` 3.0)
      (`self.CE_StartQTE`))
    (:`then_2`
      (`TimelineComponent.SetPlayRate` (`self.TL_QTEDuration`) (* (/ 1.0 (`self.SlowMotionDuration`)) (/ 1.0 (`self.ScaleTimeQTE`)))))))

(event `CE_SetTimeScale`
  (params (ScaleTime :type "Float (double-precision)"))
  ;[0.9178 1 0.515] Scale Time change
  (`GameplayStatics.SetGlobalTimeDilation` ScaleTime))

(event `CE_HandleIncibilityCooldown`
  ;[1 0.9919 0.5355] Handle Invicibility Cooldown
  (set `self.QTECurrentInvincibility` (+ (`self.QTECurrentInvincibility`) (* (`GameplayStatics.GetWorldDeltaSeconds`) (/ 1.0 (`self.ScaleTimeQTE`))))))

(event `CE_StartQTE`
  (bind _as_bp_pc_player (`self.As BP PC Player`))
  ;[1 0.972 0.3209] Start / Stop
  (`KismetSystemLibrary.PrintString` "Start QTE" true true (struct :`R` 1.0 :`G` 0.301101 :`A` 1.0))
  (`self.OnStartQTE`)
  (`self.CE_SetTimeScale` (`self.ScaleTimeQTE`))
  (set `self.QTECurrentInvincibility` 0.0)
  (set `self.HasPressedQTEKey` false)
  (set `self.HasPressedAnyKey` false)
  (`/Engine/EditorBlueprintResources/StandardMacros.IsValid` _as_bp_pc_player
    (:`Is Valid`
      (add `/Game/_Project/BP/Core/BP_PC_Player.OnPressAnyKey` _as_bp_pc_player (`|CreateDelegate` :!event `CE_CheckPressedAnyKey`))
      (set `self.IsInQTE` true)
      (`Timeline|TL_QTEDuration` :!via `PlayFromStart`
        (:`Update`
          (`self.CE_HandleIncibilityCooldown`))
        (:`Finished`
          (`self.CE_QTEOutOfTime`))))))

(event `CE_QTEOutOfTime`
  (bind _as_bp_pc_player (`self.As BP PC Player`))
  ;[1 0.6503 0.4316] Out Of time QTE
  (`/Engine/EditorBlueprintResources/StandardMacros.IsValid` _as_bp_pc_player
    (:`Is Valid`
      (clear `/Game/_Project/BP/Core/BP_PC_Player.OnPressAnyKey` _as_bp_pc_player)
      (`self.CE_LoseQTE`))))

(event `CE_StopQTE`
  (params (HasWon :type Boolean))
  ;[0.9797 1 0.3504] Stop QTE
  (set `self.IsInQTE` false)
  (`self.OnStopQTE` HasWon)
  (`self.CE_SetTimeScale` 1.0))

(event `CE_SuceedPressedQTEKey`
  (bind _as_bp_pc_player (`self.As BP PC Player`))
  ;[1 0.5713 0.1748] Handle pressed keys during QTE
  (if (`self.IsInQTE`)
    (`/Engine/EditorBlueprintResources/StandardMacros.IsValid` _as_bp_pc_player
      (:`Is Valid`
        (clear `/Game/_Project/BP/Core/BP_PC_Player.OnPressAnyKey` _as_bp_pc_player)
        (`self.CE_WinQTE`)))))

(event `CE_CheckPressedAnyKey`
  (params (KeyPressed :type "Key Structure" :default "None"))
  (bind _as_bp_pc_player (`self.As BP PC Player`))
  ;[1 0.5713 0.1748] Handle pressed keys during QTE
  (if (>= (`self.QTECurrentInvincibility`) (`self.QTEInvincibilityCooldown`))
    (if (not (== KeyPressed "LeftMouseButton"))
      (`/Engine/EditorBlueprintResources/StandardMacros.IsValid` _as_bp_pc_player
        (:`Is Valid`
          (clear `/Game/_Project/BP/Core/BP_PC_Player.OnPressAnyKey` _as_bp_pc_player)
          (`self.CE_LoseQTE`))))))

(event `CE_WinQTE`
  ;[1 0.9465 0] Win / Lose
  (`self.CE_StopQTE` true)
  (`self.OnWinQTE`)
  (`KismetSystemLibrary.PrintString` "Win QTE" true true (struct :`R` 1.0 :`G` 0.301101 :`A` 1.0)))

(event `CE_LoseQTE`
  ;[1 0.9465 0] Win / Lose
  (`self.CE_StopQTE` false)
  (`self.OnLoseQTE`)
  (`KismetSystemLibrary.PrintString` "Lose QTE" true true (struct :`R` 1.0 :`G` 0.301101 :`A` 1.0)))

(fn `UserConstructionScript`)