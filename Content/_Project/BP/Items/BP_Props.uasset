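; BP_Props is a prop item that reports itself as not catchable and gets knocked away when a catch hits it.
; The Catch event pushes its Cube mesh away from the catch location with a slight upward bias, using a random-strength velocity-change impulse that ignores mass.
; It also exposes the Cube's static mesh through GetStaticMesh.
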(event `/Game/_Project/Interfaces/I_Catchables.Catch`
  (params (CatchLocation :type "Vector Structure") (Radius :type "Float (double-precision)"))
  (bind (_returnvalue_x _returnvalue_y) (`KismetMathLibrary.BreakVector` (- (`self.K2_GetActorLocation`) CatchLocation)))
  ;[1 0.8632 0.2582] Impulse On Catch
  (`PrimitiveComponent.AddImpulse` (`self.Cube`) (* (`KismetMathLibrary.Normal` (`KismetMathLibrary.MakeVector` _returnvalue_x _returnvalue_y 100.0)) (`KismetMathLibrary.RandomFloatInRange` 300.0 500.0)) "None" true))

(fn `GetStaticMesh`
  (returns (OutStaticMesh :type "StaticMesh Object Reference"))
  (return (`StaticMeshComponent.StaticMesh` (`self.Cube`))))

(fn `IsCatchable`
  (returns (IsCatchable :type Boolean))
  (return false))

(fn `UserConstructionScript`)