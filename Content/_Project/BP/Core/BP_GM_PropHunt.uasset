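; BP_GM_PropHunt is the game mode Blueprint for Prop Hunt, owning the sound and QTE manager actors.
; Getters return the cached manager if valid, otherwise spawn BP_Manager_Sound or BP_Manager_QTE through an Init function and store the reference.
; BeginPlay calls both getters so the managers exist at game start, and any earlier request creates them lazily.
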(event `self.ReceiveBeginPlay`
  ;[0.4319 1 0.3056] Begin Play
  (`self.GetSoundManager`)
  (`self.GetQTEManager`))

(fn `GetQTEManager`
  (returns (QTEManager :type "/Game/_Project/BP/Managers/BP_Manager_QTE Object Reference"))
  (bind _qtemanager (`self.QTEManager`))
  (`/Engine/EditorBlueprintResources/StandardMacros.IsValid` _qtemanager
    (:`Is Valid`
      (return _qtemanager))
    (:`Is Not Valid`
      (bind _qtemanager_2 (`self.InitQTEManager`))
      (return _qtemanager_2))))

(fn `GetSoundManager`
  (returns (SoundManager :type "/Game/_Project/BP/Managers/BP_Manager_Sound Object Reference"))
  (bind _soundmanager (`self.SoundManager`))
  (`/Engine/EditorBlueprintResources/StandardMacros.IsValid` _soundmanager
    (:`Is Valid`
      (return _soundmanager))
    (:`Is Not Valid`
      (bind _soundmanager_2 (`self.InitSoundManager`))
      (return _soundmanager_2))))

(fn `InitQTEManager`
  (returns (QTEManager :type "/Game/_Project/BP/Managers/BP_Manager_QTE Object Reference"))
  (bind _returnvalue (`|SpawnActorFromClass` "/Game/_Project/BP/Managers/BP_Manager_QTE.BP_Manager_QTE_C" (`KismetMathLibrary.MakeTransform` (0.0 0.0 0.0)) "AlwaysSpawn" "MultiplyWithRoot" null null))
  (bind _output_get (set `self.QTEManager` _returnvalue))
  (return _output_get))

(fn `InitSoundManager`
  (returns (SoundManager :type "/Game/_Project/BP/Managers/BP_Manager_Sound Object Reference"))
  (bind _returnvalue (`|SpawnActorFromClass` "/Game/_Project/BP/Managers/BP_Manager_Sound.BP_Manager_Sound_C" (`KismetMathLibrary.MakeTransform` (0.0 0.0 0.0)) "AlwaysSpawn" "MultiplyWithRoot" null null))
  (bind _output_get (set `self.SoundManager` _returnvalue))
  (return _output_get))

(fn `UserConstructionScript`)