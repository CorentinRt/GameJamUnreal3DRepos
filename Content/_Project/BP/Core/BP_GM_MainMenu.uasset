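; Game mode for the main menu that sets up scene management and cursor-driven UI input.
; On BeginPlay it ensures a scene manager exists, then shows the mouse cursor and switches the first player controller to UI-only input.
; GetSceneManager lazily creates the manager, returning the cached reference if valid or calling InitSceneManager to spawn and store a new BP_Manager_Scene actor.
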(event `self.ReceiveBeginPlay`
  (bind _returnvalue (`GameplayStatics.GetPlayerController` 0))
  ;[0.2089 1 0.2162] Begin Play
  (`|ExecutionSequence`
    (:`then_0`
      (`self.GetSceneManager`))
    (:`then_1`
      (set `PlayerController.bShowMouseCursor` true _returnvalue)
      (`WidgetBlueprintLibrary.SetInputMode_UIOnlyEx` _returnvalue null))))

(fn `GetSceneManager`
  (returns (SceneManager :type "/Game/_Project/BP/Managers/BP_Manager_Scene Object Reference"))
  (bind _scenemanager (`self.SceneManager`))
  (`/Engine/EditorBlueprintResources/StandardMacros.IsValid` _scenemanager
    (:`Is Valid`
      (return _scenemanager))
    (:`Is Not Valid`
      (bind _scenemanager_2 (`self.InitSceneManager`))
      (return _scenemanager_2))))

(fn `InitSceneManager`
  (returns (SceneManager :type "/Game/_Project/BP/Managers/BP_Manager_Scene Object Reference"))
  (bind _returnvalue (`|SpawnActorFromClass` "/Game/_Project/BP/Managers/BP_Manager_Scene.BP_Manager_Scene_C" (`KismetMathLibrary.MakeTransform` (0.0 0.0 0.0)) "AlwaysSpawn" "MultiplyWithRoot" null null))
  (bind _output_get (set `self.SceneManager` _returnvalue))
  (return _output_get))

(fn `UserConstructionScript`)