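; Player controller Blueprint for the PropHunt game mode, handling global key and pause input.
; It caches BP_GM_PropHunt on BeginPlay and forwards pause requests to that game mode's toggle event, with a debug print.
; While unpaused, any key press is broadcast with its key through OnPressAnyKey.
; Default/QTE mapping-context switching is marked obsolete: its event is empty and the switch logic is disconnected.
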(event `self.ReceiveBeginPlay`
  ;[0.1166 1 0.2444] Begin Play
  (bind _asbp_gm_prop_hunt (cast `/Game/_Project/BP/Core/BP_GM_PropHunt` (`GameplayStatics.GetGameMode`)))
  (set `self.As BP GM Prop Hunt` _asbp_gm_prop_hunt))

(event `Key|AnyKey`
  (params (Key :type "Key Structure"))
  ;[0.2383 0.7547 1] Press Any Key
  (:`Pressed`
    (if (not (`GameplayStatics.IsGamePaused`))
      (`self.OnPressAnyKey` Key))))

(event `self.PauseReceiveInputBluePrint`
  (params (PauseValue :type "Float (single-precision)"))
  (bind _as_bp_gm_prop_hunt (`self.As BP GM Prop Hunt`))
  ;[0.381 0.8615 1] PauseGame
  (`KismetSystemLibrary.PrintString` "Pause Game")
  (`/Engine/EditorBlueprintResources/StandardMacros.IsValid` _as_bp_gm_prop_hunt
    (:`Is Valid`
      (`/Game/_Project/BP/Core/BP_GM_PropHunt.CE_TogglePause` _as_bp_gm_prop_hunt))))

(event `CE_ChangeMappingContext`
  (params (MappingContextType :type "/Game/_Project/Enums/E_MappingContextType Enum" :default "NewEnumerator0"))
  ;[1 0.8628 0] Mapping (Obsolete)
  ;;[1 0.7082 0] Change Mapping Context
)

(event `Key|Y`
  (params (Key :type "Key Structure"))
  ;[1 0.8628 0] Mapping (Obsolete)
  ;;[0.9942 1 0] Change Mapping Context
)

(event `Key|U`
  (params (Key :type "Key Structure"))
  ;[1 0.8628 0] Mapping (Obsolete)
  ;;[0.9942 1 0] Change Mapping Context
)

(fn `UserConstructionScript`)