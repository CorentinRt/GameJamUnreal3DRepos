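; Audio component for BP_Crusher that provides the grinder working and grinder end sound effects.
; On BeginPlay it casts its owner to BP_Crusher, caches it, then binds to the crusher's start and end crushing event dispatchers.
; Its two sound events spawn the matching MetaSound attached to the crusher's capsule, keeping audio logic out of the crusher Blueprint.
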(event `CE_BindSoundToCrusherEvent`
  (bind _as_bp_crusher (`self.As BP Crusher`))
  ;[0.1995 0.2294 1] Bind Sound To Crusher Event
  (`/Engine/EditorBlueprintResources/StandardMacros.IsValid` _as_bp_crusher
    (:`Is Valid`
      (add `/Game/_Project/BP/Crusher/BP_Crusher.ED_OnStartCrushing` _as_bp_crusher (`|CreateDelegate` :!event `CE_PlayGrinderWorking`))
      (add `/Game/_Project/BP/Crusher/BP_Crusher.ED_OnEndCrushing` _as_bp_crusher (`|CreateDelegate` :!event `CE_PlayGrinderEndSound`)))))

(event `CE_RecupCrusher`
  ;[0.2311 0.2414 1] Recup Crusher
  (bind _asbp_crusher (cast `/Game/_Project/BP/Crusher/BP_Crusher` (`self.GetOwner`)))
  (set `self.As BP Crusher` _asbp_crusher))

(event `self.ReceiveBeginPlay`
  ;[0.2869 1 0.4737] Begin Play
  (`|ExecutionSequence`
    (:`then_0`
      (`self.CE_RecupCrusher`))
    (:`then_1`
      (`self.CE_BindSoundToCrusherEvent`))))

(event `CE_PlayGrinderWorking`
  (bind _as_bp_crusher (`self.As BP Crusher`))
  ;[1 0.2918 0.9791] Play Grinder Working Sound
  (`/Engine/EditorBlueprintResources/StandardMacros.IsValid` _as_bp_crusher
    (:`Is Valid`
      (`GameplayStatics.SpawnSoundAttached` "/Game/_Project/Assets/Audio/SFX/Grinder/MS_SFX_GPE_GrinderWorking.MS_SFX_GPE_GrinderWorking" (`/Game/_Project/BP/Crusher/BP_Crusher.Capsule` _as_bp_crusher) "None" (0.0 0.0 0.0) (struct) "KeepRelativeOffset" true 1.0 1.0 0.0 "/Game/_Project/Audio/Attenuationprofiles/SA_Props.SA_Props" null))))

(event `CE_PlayGrinderEndSound`
  (bind _as_bp_crusher (`self.As BP Crusher`))
  ;[1 0.2518 0.9921] Play Grinder End Sound
  (`/Engine/EditorBlueprintResources/StandardMacros.IsValid` _as_bp_crusher
    (:`Is Valid`
      (`GameplayStatics.SpawnSoundAttached` "/Game/_Project/Assets/Audio/SFX/Grinder/MS_SFX_GPE_GrinderEnd.MS_SFX_GPE_GrinderEnd" (`/Game/_Project/BP/Crusher/BP_Crusher.Capsule` _as_bp_crusher) "None" (0.0 0.0 0.0) (struct) "KeepRelativeOffset" true 1.0 1.0 0.0 "/Game/_Project/Audio/Attenuationprofiles/SA_Props.SA_Props" null))))