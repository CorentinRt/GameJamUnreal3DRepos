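; BP_Crusher is a crusher actor where players dispose of carried SCPs in the prop hunt game mode.
; On begin play it caches the prop hunt game mode.
; When a player character carrying an SCP overlaps it, it destroys that SCP, clears the player's carrying state and tells the game mode to decrease the count of SCPs left to find.
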(event `self.ReceiveBeginPlay`
  ;[0.2103 1 0.4218] Begin Play
  (bind _asbp_gm_prop_hunt (cast `/Game/_Project/BP/Core/BP_GM_PropHunt` (`GameplayStatics.GetGameMode`)))
  (set `self.As BP GM Prop Hunt` _asbp_gm_prop_hunt))

(event `self.ReceiveActorBeginOverlap`
  (params (OtherActor :type "Actor Object Reference"))
  (bind _as_bp_gm_prop_hunt (`self.As BP GM Prop Hunt`))
  ;[1 0.009508 0] Player Overlap Crusher
  (bind _asbp_chara_player (cast `/Game/_Project/BP/Player/BP_Chara_Player` OtherActor))
  (if (`/Game/_Project/BP/Player/BP_Chara_Player.IsCarryingScp` _asbp_chara_player)
    (`self.K2_DestroyActor` (`/Game/_Project/BP/Player/BP_Chara_Player.SCPCarried` _asbp_chara_player))
    (`/Game/_Project/BP/Player/BP_Chara_Player.CE_TriggerIsCarryingScp` _asbp_chara_player false)
    (`/Engine/EditorBlueprintResources/StandardMacros.IsValid` _as_bp_gm_prop_hunt
      (:`Is Valid`
        (`/Game/_Project/BP/Core/BP_GM_PropHunt.DecreaseSCPToFind` _as_bp_gm_prop_hunt)))))

(fn `UserConstructionScript`)