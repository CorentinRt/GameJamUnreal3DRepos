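; Player character Blueprint for a prop hunt game, handling the catch action and caching the game mode on begin play.
; Catching line-traces along the camera's forward vector, sphere-traces around the impact, sends CatchMessage to I_Catchables actors found, then shakes the camera.
; C and V keys switch random character movement on and off with debug prints.
; The QTE action is a stub that only prints and checks its manager's validity.
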(event `self.ReceiveBeginPlay`
  ;[0.2037 1 0.304] Begin Play
  (`|ExecutionSequence`
    (:`then_0`
      (bind _asbp_gm_prop_hunt (cast `/Game/_Project/BP/Core/BP_GM_PropHunt` (`GameplayStatics.GetGameMode`)))
      (set `self.As BP GM Prop Hunt` _asbp_gm_prop_hunt))))

(event `self.CatchActionBlueprint`
  (params (CatchValue :type "Float (single-precision)"))
  ;[1 0.8632 0.2582] Catch Action Blueprint
  (`|ExecutionSequence`
    (:`then_0`
      (bind (_outhit _returnvalue) (`KismetSystemLibrary.LineTraceSingle` :`Start` (`self.K2_GetActorLocation`) :`End` (+ (`self.K2_GetActorLocation`) (* (`SceneComponent.GetForwardVector` (`self.CameraComponent`)) 800.0)) :`TraceChannel` "TraceTypeQuery1" :`DrawDebugType` "ForDuration" :`DrawTime` 2.0))
      (if _returnvalue
        (bind (_bblockinghit _binitialoverlap _time _distance _location) (`GameplayStatics.BreakHitResult` _outhit))
        (bind (_outhits _returnvalue_2) (`KismetSystemLibrary.SphereTraceMultiForObjects` :`Start` _location :`End` _location :`Radius` 100.0 :`ObjectTypes` (`|MakeArray` "ObjectTypeQuery8" :!type "EObjectTypeQuery Enum") :`DrawDebugType` "ForDuration" :`DrawTime` 1.0))
        (if _returnvalue_2
          (for _array_element _outhits
            (bind (_bblockinghit_2 _binitialoverlap_2 _time_2 _distance_2 _location_2 _impactpoint _normal _impactnormal _physmat _hitactor) (`GameplayStatics.BreakHitResult` _array_element))
            (if (`KismetSystemLibrary.DoesImplementInterface` _hitactor "/Game/_Project/Interfaces/I_Catchables.I_Catchables_C")
              (message `/Game/_Project/Interfaces/I_Catchables.Catch` _hitactor _location))))))
    (:`then_1`
      (`PlayerCameraManager.StartCameraShake` :`self` (`GameplayStatics.GetPlayerCameraManager` 0) :`ShakeClass` "/Game/_Project/BP/CameraShakes/BP_CatchCameraShake.BP_CatchCameraShake_C"))))

(event `Key|C`
  (params (Key :type "Key Structure"))
  (:`Pressed`
    (`self.SetCharacterRandomMovement` true)
    (`KismetSystemLibrary.PrintString` "Random")))

(event `Key|V`
  (params (Key :type "Key Structure"))
  (:`Pressed`
    (`self.SetCharacterRandomMovement` false)
    (`KismetSystemLibrary.PrintString` "NotRandom")))

(event `self.QTEActionBlueprint`
  (params (QTEValue :type "Float (single-precision)"))
  (`KismetSystemLibrary.PrintString` "QTE" true true (struct :`R` 1.0 :`B` 0.681815 :`A` 1.0))
  (`/Engine/EditorBlueprintResources/StandardMacros.IsValid` (`self.BP_Mananger_QTE`)))

(fn `UserConstructionScript`)