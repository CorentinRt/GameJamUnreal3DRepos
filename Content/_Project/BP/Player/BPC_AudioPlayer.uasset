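; Player audio component that plays hand and walking sound effects attached to the owning BP_Chara_Player's capsule.
; On BeginPlay it caches the owner and binds to its catch-action and catch-hit-ground dispatchers, alongside events for woosh and hit sounds.
; Tick drives footsteps while grounded, using a Delay to throttle repeats and scaling volume by velocity relative to max walk speed.
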(event `CE_BindSoundToPlayerEvents`
  (bind _as_bp_chara_player (`self.As BP Chara Player`))
  ;[0.28 0.3867 1] Bind Sound To Player Events
  (`/Engine/EditorBlueprintResources/StandardMacros.IsValid` _as_bp_chara_player
    (:`Is Valid`
      (add `/Game/_Project/BP/Player/BP_Chara_Player.ED_OnCatchAction` _as_bp_chara_player (`|CreateDelegate` :!event `CE_PlayHandWooshSound`))
      (add `/Game/_Project/BP/Player/BP_Chara_Player.ED_OnCatchHitGround` _as_bp_chara_player (`|CreateDelegate` :!event `CE_PlayHandHitSound`)))))

(event `CE_RecupPlayer`
  ;[0.3484 0.4888 1] Recup Player
  (bind _asbp_chara_player (cast `/Game/_Project/BP/Player/BP_Chara_Player` (`self.GetOwner`)))
  (set `self.As BP Chara Player` _asbp_chara_player))

(event `self.ReceiveBeginPlay`
  ;[0.2916 1 0.2665] Begin Play
  (`|ExecutionSequence`
    (:`then_0`
      (`self.CE_RecupPlayer`))
    (:`then_1`
      (`self.CE_BindSoundToPlayerEvents`))))

(event `self.ReceiveTick`
  (params (DeltaSeconds :type "Float (single-precision)"))
  ;[1 0.1421 0] Tick
  (`self.CE_HandleWalkSound`))

(event `CE_PlayHandHitSound`
  (bind _as_bp_chara_player (`self.As BP Chara Player`))
  ;[1 0.4696 0.9436] Play Hit Sound
  (`/Engine/EditorBlueprintResources/StandardMacros.IsValid` _as_bp_chara_player
    (:`Is Valid`
      (`GameplayStatics.SpawnSoundAttached` "/Game/_Project/Assets/Audio/SFX/Hand/MS_SFX_GPE_HandHit.MS_SFX_GPE_HandHit" (`Character.CapsuleComponent` _as_bp_chara_player) "None" (0.0 0.0 0.0) (struct) "KeepRelativeOffset" true 1.0 1.0 0.0 null null))))

(event `CE_PlayHandWooshSound`
  (bind _as_bp_chara_player (`self.As BP Chara Player`))
  ;[1 0.4086 0.9] Play Hand Woosh Sound
  (`/Engine/EditorBlueprintResources/StandardMacros.IsValid` _as_bp_chara_player
    (:`Is Valid`
      (`GameplayStatics.SpawnSoundAttached` "/Game/_Project/Assets/Audio/SFX/Hand/MS_SFX_GPE_HandWoosh.MS_SFX_GPE_HandWoosh" (`Character.CapsuleComponent` _as_bp_chara_player) "None" (0.0 0.0 0.0) (struct) "KeepRelativeOffset" true 1.0 1.0 0.0 null null))))

(event `CE_HandleWalkSound`
  (bind _as_bp_chara_player (`self.As BP Chara Player`))
  (bind _charactermovement (`Character.CharacterMovement` _as_bp_chara_player))
  ;[1 0.3338 0.8532] Handle Walking Sound
  (`/Engine/EditorBlueprintResources/StandardMacros.IsValid` _as_bp_chara_player
    (:`Is Valid`
      (if (`NavMovementComponent.IsMovingOnGround` _charactermovement)
        (`KismetSystemLibrary.Delay` 0.3)
        (`GameplayStatics.SpawnSoundAttached` "/Game/_Project/Assets/Audio/SFX/Walking/MS_SFX_GPE_Walking.MS_SFX_GPE_Walking" (`Character.CapsuleComponent` _as_bp_chara_player) "None" (0.0 0.0 0.0) (struct) "KeepRelativeOffset" true (/ (`KismetMathLibrary.VSize` (`MovementComponent.Velocity` _charactermovement)) (`CharacterMovementComponent.MaxWalkSpeed` _charactermovement)) 1.0 0.0 null null)))))