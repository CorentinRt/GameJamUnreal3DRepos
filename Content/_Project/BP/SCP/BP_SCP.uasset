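; SCP for a prop-hunt mode that hides by possessing props and exposes itself through randomly chosen hint components, with a looping hint timer.
; A catch attempt is graded by distance: close catches it, mid-range starts a QTE, farther only prints a hint message.
; A lost QTE spawns a fleeing actor.
; When the flee ends, a sphere trace picks a free prop behind the player, falling back to any free prop.
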(event `self.ReceiveBeginPlay`)

(event `OnFleeEndEvent`
  (params (EndPos :type "Vector Structure"))
  (`self.TeleportToNewLocation` EndPos))

(event `OnStopQTEEvent`
  (params (HasWon :type Boolean))
  (if HasWon
    (`KismetSystemLibrary.PrintString` "SPC Was catched !")
    (else
      (`KismetSystemLibrary.PrintString` "Flee")
      (`self.Flee`))))

(fn `Catch`
  (params (CatchLocation :type "Vector Structure") (Radius :type "Float (double-precision)"))
  (returns (HasBeenCaught :type Boolean) (ActorRef :type "Actor Object Reference"))
  (bind _hasbeencatch (`self.Check Catch Distance` CatchLocation Radius))
  (return _hasbeencatch self))

(fn `Check Catch Distance`
  (params (CatchLocation :type "Vector Structure") (CatchRadius :type "Float (double-precision)"))
  (returns (HasBeenCatch :type Boolean))
  (locals (DistanceToCatchPoint :type "Float (double-precision)"))
  (bind _returnvalue (/ (`local.CatchRadius`) 3.0))
  ;[1 1 1] Get Distance with catch point
  (set `local.DistanceToCatchPoint` (`KismetMathLibrary.Vector_Distance` CatchLocation (`self.K2_GetActorLocation` (`self.PossessedProps`))))
  (if (<= (`local.DistanceToCatchPoint`) _returnvalue)
    (set `self.IsCatchable?` false)
    (`self.UnpossessCurrentProps`)
    (`KismetSystemLibrary.PrintString` "Catch")
    (return true)
    (elif (<= (`local.DistanceToCatchPoint`) (* _returnvalue 2.0))
      (set `self.IsCatchable?` false)
      (`self.UnpossessCurrentProps`)
      (`KismetSystemLibrary.PrintString` "TryToFlee")
      (`self.TryToFlee`)
      (return false)
      (else
        (`KismetSystemLibrary.PrintString` "Hint")
        (return false)))))

(fn `CheckForPropsBehindPlayer`
  (params (SphereCastStart :type "Vector Structure"))
  (returns (OutValidProps :type "Array of /Game/_Project/BP/Items/BP_Props Object Reference") (FoundValidProps :type Boolean))
  (locals (ValidProps :type "Array of /Game/_Project/BP/Items/BP_Props Object Reference") (PlayerForwardVector :type "Vector Structure") (PlayerLocation :type "Vector Structure"))
  (bind _returnvalue (`GameplayStatics.GetPlayerPawn` 0))
  (bind _validprops (`local.ValidProps`))
  ;[1 1 1] Check if we hit any object with the "props" trace profile in blocking
  (bind _outhits (`KismetSystemLibrary.SphereTraceMulti` :`Start` SphereCastStart :`End` SphereCastStart :`Radius` (`self.TeleportSphereCastRadius`) :`TraceChannel` "TraceTypeQuery3" :`DrawDebugType` "Persistent"))
  (if (> (`KismetArrayLibrary.Array_Length` _outhits) 0)
    (set `local.PlayerLocation` (`self.K2_GetActorLocation` _returnvalue))
    (set `local.PlayerForwardVector` (`self.GetActorForwardVector` _returnvalue))
    (for _array_element _outhits
      (bind (_bblockinghit _binitialoverlap _time _distance _location _impactpoint _normal _impactnormal _physmat _hitactor) (`GameplayStatics.BreakHitResult` _array_element))
      ;[1 1 1] Verify that props is a valid props to tp to (right object class & behind player)
      (bind _asbp_props (cast `/Game/_Project/BP/Items/BP_Props` _hitactor)
        (:`then`
          _)
        (:`CastFailed`
          _))
      (if (and (not (`/Game/_Project/BP/Items/BP_Props.IsPossessed?` _asbp_props)) (== (`GameplayStatics.GetObjectClass` _hitactor) "/Game/_Project/BP/Items/BP_Props.BP_Props_C") (< (`KismetMathLibrary.Dot_VectorVector` (`KismetMathLibrary.Normal` (- (`self.K2_GetActorLocation` _hitactor) (`local.PlayerLocation`))) (`local.PlayerForwardVector`)) 0.0))
        (bind _asbp_props_2 (cast `/Game/_Project/BP/Items/BP_Props` _hitactor))
        (`KismetArrayLibrary.Array_Add` (`local.ValidProps`) _asbp_props_2)))
    (return _validprops (> (`KismetArrayLibrary.Array_Length` _validprops) 0))
    (else
      (return (`local.ValidProps`) false))))

(fn `Flee`
  (`self.K2_DetachFromActor` "KeepRelative")
  ;[1 1 1] Spawn Flee Actor
  (bind _returnvalue (`|SpawnActorFromClass` "/Game/_Project/BP/SCP/BP_FleeingSCP.BP_FleeingSCP_C" (`self.GetTransform`) "Undefined" "MultiplyWithRoot" null null))
  (bind _output_get (set `self.FleeingSCP` _returnvalue))
  (add `/Game/_Project/BP/SCP/BP_FleeingSCP.FleeEndEvent` _output_get (`|CreateDelegate` :!event `OnFleeEndEvent`))
  (`/Game/_Project/BP/SCP/BP_FleeingSCP.DoFleeAnimation` _output_get))

(fn `GetHintTime`
  (returns (OutHintTime :type "Float (double-precision)"))
  (return (`self.HintTime`)))

(fn `GiveHint`
  (locals (ActivablesHints :type "Array of /Game/_Project/BP/SCP/SCPHints/BP_SCPHint Object Reference"))
  (bind _activableshints (`local.ActivablesHints`))
  (bind _returnvalue (`KismetArrayLibrary.Array_Length` _activableshints))
  (if (`KismetSystemLibrary.IsValid` (`self.PossessedProps`))
    (for _array_element (`self.SCPHints`)
      (if (`/Game/_Project/BP/SCP/SCPHints/BP_SCPHint.IsActivable` _array_element)
        (`KismetArrayLibrary.Array_Add` (`local.ActivablesHints`) _array_element)))
    (if (> _returnvalue 0)
      (`/Game/_Project/BP/SCP/SCPHints/BP_SCPHint.ActivateHint` (`|GetArrayItem` _activableshints (`KismetMathLibrary.RandomInteger` _returnvalue)))
      (else
        (`KismetSystemLibrary.PrintString` "NO ACTIVABLE HINTS" true true (struct :`R` 1.0 :`G` 0.175961 :`A` 1.0))))
    (else
      (`KismetSystemLibrary.PrintString` "No Props to give hint" true true (struct :`R` 1.0 :`B` 0.029016 :`A` 1.0)))))

(fn `Init`
  ;[1 1 1] Init Hint Comps
  (for _array_element (`self.K2_GetComponentsByClass` "/Game/_Project/BP/SCP/SCPHints/BP_SCPHint.BP_SCPHint_C")
    (`/Game/_Project/BP/SCP/SCPHints/BP_SCPHint.InitHint` _array_element self)
    (`KismetArrayLibrary.Array_Add` (`self.SCPHints`) _array_element))
  (bind _returnvalue (`KismetSystemLibrary.K2_SetTimerDelegate` (`|CreateDelegate` :!event `GiveHint`) (`self.HintTime`) true))
  (set `self.HintTimerHandle` _returnvalue)
  (bind _asbp_gm_prop_hunt (cast `/Game/_Project/BP/Core/BP_GM_PropHunt` (`GameplayStatics.GetGameMode`)))
  (bind _outprops (`/Game/_Project/BP/Core/BP_GM_PropHunt.GetRandomUnpossessedProps` _asbp_gm_prop_hunt))
  (`self.PossessNewProps` _outprops))

(fn `IsCatchable`
  (returns (IsCatchable :type Boolean))
  (return (`self.IsCatchable?`)))

(fn `PossessNewProps`
  (params (PropsToPossess :type "/Game/_Project/BP/Items/BP_Props Object Reference"))
  (returns (PossessedNewProps :type Boolean))
  (bind _output_get (set `self.PossessedProps` PropsToPossess))
  (`/Game/_Project/BP/Items/BP_Props.Possess` _output_get self)
  (`BlendSpaceLibrary.SnapToPosition` (`self.SnapBlendSpace`) (`self.K2_GetActorLocation` (`self.PossessedProps`)))
  (`self.K2_AttachToActor` (`self.PossessedProps`) "None" "KeepRelative" "KeepRelative" "KeepRelative")
  (set `self.IsCatchable?` true)
  (return true))

(fn `TeleportToNewLocation`
  (params (SphereCastStart :type "Vector Structure") (UseAllRoom :type Boolean))
  (if UseAllRoom
    (bind _asbp_gm_prop_hunt (cast `/Game/_Project/BP/Core/BP_GM_PropHunt` (`GameplayStatics.GetGameMode`)))
    (bind _outprops (`/Game/_Project/BP/Core/BP_GM_PropHunt.GetRandomUnpossessedProps` _asbp_gm_prop_hunt))
    (bind _possessednewprops (`self.PossessNewProps` _outprops))
    (if _possessednewprops
      (`KismetSystemLibrary.PrintString` "Success All Room")
      (else
        (`KismetSystemLibrary.PrintString` "Failed All Room")))
    (else
      (bind (_outvalidprops _foundvalidprops) (`self.CheckForPropsBehindPlayer` SphereCastStart))
      (if _foundvalidprops
        (bind _possessednewprops_2 (`self.PossessNewProps` (`|GetArrayItem` _outvalidprops (`KismetMathLibrary.RandomInteger` (`KismetArrayLibrary.Array_Length` _outvalidprops)))))
        (if _possessednewprops_2
          (set `self.IsCatchable?` true)
          (`KismetSystemLibrary.PrintString` "TELEPORT" true true (struct :`R` 1.0 :`B` 0.800638 :`A` 1.0))
          (else
            (`KismetSystemLibrary.PrintString` "FAILED TO TELEPORT" true true (struct :`R` 1.0 :`B` 0.800638 :`A` 1.0))))
        (else
          (`self.TeleportToNewLocation` (0.0 0.0 0.0) true))))))

(fn `TryToFlee`
  (bind _asbp_gm_prop_hunt (cast `/Game/_Project/BP/Core/BP_GM_PropHunt` (`GameplayStatics.GetGameMode`)))
  (bind _qtemanager (`/Game/_Project/BP/Core/BP_GM_PropHunt.GetQTEManager` _asbp_gm_prop_hunt))
  (add `/Game/_Project/BP/Managers/BP_Manager_QTE.OnStopQTE` _qtemanager (`|CreateDelegate` :!event `OnStopQTEEvent`))
  (`/Game/_Project/BP/Managers/BP_Manager_QTE.CE_StartQTE` _qtemanager))

(fn `UnpossessCurrentProps`
  (`/Game/_Project/BP/Items/BP_Props.Unpossess` (`self.PossessedProps`))
  (`self.K2_DetachFromActor` "KeepRelative")
  (set `self.PossessedProps` null))

(fn `UserConstructionScript`)