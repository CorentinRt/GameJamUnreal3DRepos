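; SCP hint that slides the SCP's possessed prop across the world while it is out of the player's view.
; Activation requires a valid, recently unrendered prop, then picks a random horizontal direction and starts a timer slightly shorter than the SCP's hint time.
; Tick moves the prop at MoveSpeed without sweeping, stopping the hint and clearing the timer once the prop is rendered or invalid.
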(event `self.ReceiveTick`
  (params (DeltaSeconds :type "Float (single-precision)"))
  (bind _possessedprops (`/Game/_Project/BP/SCP/BP_SCP.PossessedProps` (`self.SCP`)))
  (if (`self.IsActivated`)
    (if (and (not (`Actor.WasRecentlyRendered` _possessedprops 0.2)) (`KismetSystemLibrary.IsValid` _possessedprops))
      (`self.MoveSelfProps` DeltaSeconds)
      (else
        (`self.StopHint`)))))

(fn `ActivateHint`
  (bind (_returnvalue_x _returnvalue_y) (`KismetMathLibrary.BreakVector` (`KismetMathLibrary.RandomUnitVector`)))
  (`parent.ActivateHint`)
  (set `self.MoveDirection` (`KismetMathLibrary.Normal` (`KismetMathLibrary.MakeVector` _returnvalue_x _returnvalue_y)))
  (bind _returnvalue (`KismetSystemLibrary.K2_SetTimerDelegate` (`|CreateDelegate` :!event `StopHint`) (- (`/Game/_Project/BP/SCP/BP_SCP.GetHintTime` (`self.SCP`)) 0.1)))
  (set `self.StopTimerHandle` _returnvalue))

(fn `IsActivable`
  (returns (IsActivable :type Boolean))
  (bind _possessedprops (`/Game/_Project/BP/SCP/BP_SCP.PossessedProps` (`self.SCP`)))
  (return (and (`KismetSystemLibrary.IsValid` _possessedprops) (not (`Actor.WasRecentlyRendered` _possessedprops 0.1)))))

(fn `MoveSelfProps`
  (params (DeltaSeconds :type "Float (double-precision)"))
  (`/Engine/EditorBlueprintResources/StandardMacros.IsValid` (`/Game/_Project/BP/SCP/BP_SCP.PossessedProps` (`self.SCP`))
    (:`Is Valid`
      (`Actor.K2_SetActorLocation` (`/Game/_Project/BP/SCP/BP_SCP.PossessedProps` (`self.SCP`)) (+ (* (* (`self.MoveDirection`) (`self.MoveSpeed`)) (`local.DeltaSeconds`)) (`Actor.K2_GetActorLocation` (`/Game/_Project/BP/SCP/BP_SCP.PossessedProps` (`self.SCP`)))) false false))))

(fn `StopHint`
  (`parent.StopHint`)
  (`KismetSystemLibrary.K2_ClearAndInvalidateTimerHandle` (`self.StopTimerHandle`)))