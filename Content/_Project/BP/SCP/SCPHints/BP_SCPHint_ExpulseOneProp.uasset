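; BP_SCPHint_ExpulseOneProp is an SCP hint that flings one nearby prop to betray the SCP's presence.
; ActivateHint sphere-traces around the owner within ActionRadius, ignoring the SCP's possessed props, and picks one random hit.
; If that hit is a BP_Props, its mesh receives a mass-independent impulse in a random upper-hemisphere direction, scaled by ImpulseStrength.
; A non-prop pick does nothing, and the parent ActivateHint is never called.
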(fn `ActivateHint`
  (bind _returnvalue (`Actor.K2_GetActorLocation` (`self.GetOwner`)))
  (bind _outhits (`KismetSystemLibrary.SphereTraceMulti` _returnvalue _returnvalue (`self.ActionRadius`) "TraceTypeQuery3" false (`|MakeArray` (`/Game/_Project/BP/SCP/BP_SCP.PossessedProps` (`self.SCP`)) :!type "Actor Object Reference")))
  (bind _returnvalue_2 (`KismetArrayLibrary.Array_Length` _outhits))
  (if (> _returnvalue_2 0)
    (bind _asbp_props (cast `/Game/_Project/BP/Items/BP_Props` (`.HitActor` (`GameplayStatics.BreakHitResult` (`|GetArrayItem` _outhits (`KismetMathLibrary.RandomInteger` _returnvalue_2))))))
    (`PrimitiveComponent.AddImpulse` (`/Game/_Project/BP/Items/BP_Props.PropsMesh` _asbp_props) (* (`KismetMathLibrary.RandomUnitVectorInConeInDegrees` (0.0 0.0 1.0) 90.0) (`self.ImpulseStrength`)) "None" true)))