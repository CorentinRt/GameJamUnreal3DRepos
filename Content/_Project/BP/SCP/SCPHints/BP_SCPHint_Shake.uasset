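; SCP hint that makes the SCP's possessed prop shake while the hint is active.
; On activation it saves the prop's transform and sets a one-shot timer to the shorter of its shaking time and the SCP's hint time.
; Tick nudges the prop in random directions with swept moves scaled by delta time, so offsets accumulate.
; Stopping clears the timer and restores the saved transform.
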(event `self.ReceiveTick`
  (params (DeltaSeconds :type "Float (single-precision)"))
  (if (`self.IsActivated`)
    (`self.Shake` DeltaSeconds)))

(fn `ActivateHint`
  (bind _shakingtime (`self.ShakingTime`))
  (bind _outhinttime (`/Game/_Project/BP/SCP/BP_SCP.GetHintTime` (`self.SCP`)))
  (`parent.ActivateHint`)
  (set `self.StartTransform` (`Actor.GetTransform` (`/Game/_Project/BP/SCP/BP_SCP.PossessedProps` (`self.SCP`))))
  (bind _returnvalue (`KismetSystemLibrary.K2_SetTimerDelegate` (`|CreateDelegate` :!event `StopHint`) (`KismetMathLibrary.SelectFloat` _shakingtime _outhinttime (< _shakingtime _outhinttime))))
  (set `self.ShakingTimerHandle` _returnvalue))

(fn `Shake`
  (params (DeltaSeconds :type "Float (double-precision)"))
  (`Actor.K2_SetActorLocation` (`/Game/_Project/BP/SCP/BP_SCP.PossessedProps` (`self.SCP`)) (+ (* (* (`KismetMathLibrary.RandomUnitVector`) (`self.ShakeDistance`)) (`local.DeltaSeconds`)) (`Actor.K2_GetActorLocation` (`/Game/_Project/BP/SCP/BP_SCP.PossessedProps` (`self.SCP`)))) true false))

(fn `StopHint`
  (`parent.StopHint`)
  (`KismetSystemLibrary.K2_ClearAndInvalidateTimerHandle` (`self.ShakingTimerHandle`))
  (`Actor.K2_SetActorTransform` (`/Game/_Project/BP/SCP/BP_SCP.PossessedProps` (`self.SCP`)) (`self.StartTransform`) false false))