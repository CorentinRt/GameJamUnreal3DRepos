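; BP_FleeingSCP is an SCP actor that plays a one-shot flee movement past the player, then destroys itself.
; DoFleeAnimation sets an end point behind the player along the actor-to-player line and scales a timeline's play rate by AnimationTime.
; The timeline lerps position while adding a curve-driven offset along a random direction within a cone around the travel direction.
; On finish it fires the flee-end event with the end location.
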(event `self.ReceiveBeginPlay`
  (set `self.PlayerPawn` (`GameplayStatics.GetPlayerPawn` 0)))

(event `DoFleeAnimation`
  (set `self.StartLocation` (`self.K2_GetActorLocation`))
  (`self.CalculateEndLocation`)
  (set `self.OffserDirection` (`KismetMathLibrary.RandomUnitVectorInConeInDegrees` (- (`self.EndLocation`) (`self.StartLocation`)) 60.0))
  (`TimelineComponent.SetPlayRate` (`self.PosTimeline`) (/ 1.0 (`self.AnimationTime`)))
  (bind (_direction _position _offset) (`Timeline|PosTimeline` :!via `PlayFromStart`)
    (:`Update`
      (`self.K2_SetActorLocation` (+ (`KismetMathLibrary.VLerp` (`self.StartLocation`) (`self.EndLocation`) _position) (* (`self.OffserDirection`) (`KismetMathLibrary.Lerp` 0.0 (`self.MaxCurveOffset`) _offset)))))
    (:`Finished`
      (`self.FleeEndEvent` (`self.EndLocation`))
      (`self.K2_DestroyActor`))))

(fn `CalculateEndLocation`
  (`/Engine/EditorBlueprintResources/StandardMacros.IsValid` (`self.PlayerPawn`)
    (:`Is Valid`
      (set `self.EndLocation` (+ (`self.K2_GetActorLocation` (`self.PlayerPawn`)) (* (`KismetMathLibrary.Normal` (- (`self.K2_GetActorLocation` (`self.PlayerPawn`)) (`self.K2_GetActorLocation`))) (`self.OffsetBehindPlayer`)))))
    (:`Is Not Valid`
      (`KismetSystemLibrary.PrintString` "No valid player for scp end pos calculation" true true (struct :`R` 1.0 :`B` 0.023769 :`A` 1.0)))))

(fn `UserConstructionScript`)